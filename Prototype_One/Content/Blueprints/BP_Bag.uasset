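; BP_Bag is a bag actor that leaves a drag trail when its weight reaches PlayerWeightThreshold.
; Each Tick at that weight, it writes its location to the EntityPositions material parameter collection as bagGroundPos for materials to read.
; After moving over 10 units from the last stored position, it waits briefly, spawns a BP_DragPrefab yawed along the movement direction, then stores the new position.
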(event `self.ReceiveTick`
  (params (DeltaSeconds :type "Float (single-precision)"))
  (bind _returnvalue (`self.K2_GetActorLocation`))
  (bind _returnvalue_2 (- _returnvalue (`self.LaastPos`)))
  (bind (_returnvalue_roll _returnvalue_pitch _returnvalue_yaw) (`KismetMathLibrary.BreakRotator` (`KismetMathLibrary.FindLookAtRotation` (`self.K2_GetActorLocation`) (+ _returnvalue _returnvalue_2))))
  (`|ExecutionSequence`
    (:`then_0`
      (bind _returnvalue_3 (`self.GetWeight`))
      (if (>= _returnvalue_3 (`self.PlayerWeightThreshold`))
        (`KismetMaterialLibrary.SetVectorParameterValue` "/Game/Environment/EntityPositions.EntityPositions" "bagGroundPos" (`KismetMathLibrary.Conv_VectorToLinearColor` (`self.K2_GetActorLocation`)))))
    (:`then_1`
      (bind _returnvalue_4 (`self.GetWeight`))
      (if (and (>= _returnvalue_4 (`self.PlayerWeightThreshold`)) (> (`KismetMathLibrary.VSize` _returnvalue_2) 10.0))
        (`KismetSystemLibrary.Delay` 0.2)
        (`|SpawnActorFromClass` "/Game/Blueprints/BP_DragPrefab.BP_DragPrefab_C" (`KismetMathLibrary.MakeTransform` (`self.K2_GetActorLocation`) (`KismetMathLibrary.MakeRotator` 0.0 0.0 _returnvalue_yaw)) "Undefined" "OverrideRootScale" null null)
        (set `self.LaastPos` _returnvalue)))))

(fn `UserConstructionScript`)